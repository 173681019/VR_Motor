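; Spline actor that carries a configurable static mesh, set up to move it along its spline.
; The construction script assigns the mesh, and BeginPlay derives a play rate from Speed divided by spline length.
; A timeline update would place and rotate the mesh along the spline with a yaw offset and apply that rate.
; Nothing triggers the timeline, so the movement never runs from this graph.
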(event Collision|EventActorBeginOverlap
  (params (OtherActor :type Actor%20Object%20Reference)))

(event EventTick
  (params (DeltaSeconds :type Float%20%28single-precision%29)))

(event EventBeginPlay
  (bind _output_get (Variables|Default|SetDefaultRate (/ (Variables|Default|GetSpeed) (Spline|GetSplineLength (Variables|Default|GetSpline)))))
  (Variables|Default|SetRate _output_get))

(fn ConstructionScript
  (Components|StaticMesh|SetStaticMesh (Variables|Default|GetStaticMesh) (Variables|Default|GetMesh)))