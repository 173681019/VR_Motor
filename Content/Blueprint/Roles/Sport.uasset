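; Player motorbike pawn for VR with chase and in-vehicle cameras, throwable props and hurt/slow hit effects.
; Input drives vehicle movement and timeline-blended steering and rider lean, while Tick updates parking thrust, slowdown, speed HUD and hands.
; Controller hands near handlebar sockets swap to bike-mounted hands; sustained fast swings within a camera-forward angle launch held banana, slow or hammer props.
; Paired Server/Client events relay steering, hands, effects and firing for multiplayer.
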(event Custom|MoveRight_S
  (params (AxisValue :type Float%20%28single-precision%29))
  ;[0.3937 1 0.39] Move Left/Right
  (CallFunction|MoveRightC AxisValue))

(event Custom|LightServer
  (params (Visivility :type Boolean))
  ;[1 1 1] 车灯
  (CallFunction|LoghtCLient Visivility))

(event Custom|HurtServer
  ;[1 1 1] stop move
  (CallFunction|HurtClient))

(event Custom|HurtClient
  (bind _vehiclemovement (Variables|Default|GetVehicleMovement))
  (bind _vehiclemovement_2 (Variables|Default|GetVehicleMovement))
  (bind _updatedprimitive (Variables|/Script/Engine.MovementComponent|GetUpdatedPrimitive _vehiclemovement))
  ;[1 1 1] stop move
  (if (Variables|Default|Gethurt？)
    (CallFunction|PrintP "已在旋转中")
    (else
      (Variables|Default|Sethurt？ true)
      (Components|Movement|StopMovementImmediately _vehiclemovement_2)
      (Class|WheeledVehicleMovementComponent|SetHandbrakeInput _vehiclemovement_2 true)
      (Class|PrimitiveComponent|SetAllPhysicsLinearVelocity (Variables|/Script/Engine.MovementComponent|GetUpdatedPrimitive _vehiclemovement_2) "0, 0,200.000000" false)
      ;[1 1 1] 眩晕
      (Components|Activation|SetActive (Variables|Default|GetPhysicsThruster) true false)
      (Utilities|FlowControl|Delay 0.4)
      (Components|Activation|SetActive (Variables|Default|GetPhysicsThruster) false false)
      (Utilities|FlowControl|Delay 1.6)
      (Class|PrimitiveComponent|SetAllPhysicsLinearVelocity _updatedprimitive "0, 0, 0" false)
      (Class|PrimitiveComponent|SetPhysicsAngularVelocityinRadians _updatedprimitive "0, 0, 0" false "None")
      (Class|WheeledVehicleMovementComponent|SetHandbrakeInput _vehiclemovement false)
      (Variables|Default|Sethurt？ false))))

(event Custom|LoghtClient
  (params (Visivility :type Boolean))
  ;[1 1 1] 车灯
  (Rendering|SetVisibility (Variables|Default|GetSpotLightRight) Visivility false))

(event Custom|Reset%20VR%20Device
  ;[1 1 1] 重置镜头
  (Class|HeadMountedDisplayFunctionLibrary|ResetOrientationandPosition 0.0 "OrientationAndPosition"))

(event Custom|MoveRight_C
  (params (AxisValue :type Float%20%28single-precision%29))
  ;[0.3937 1 0.39] Move Left/Right
  (Class|WheeledVehicleMovementComponent|SetSteeringInput (Variables|Default|GetVehicleMovement) AxisValue)
  (Utilities|FlowControl|Sequence
    (:then_0
      (if (> AxisValue 0.1)
        (Utilities|FlowControl|Sequence
          (:then_0
            (bind _newtrack_0 (Timeline|Timeline_3 PlayFromStart)
              (:Update
                (Variables|Moto|SetSteer (Math|Rotator|Lerp(Rotator) (Variables|Moto|GetSteer) "0, 0,25.000000" _newtrack_0)))))
          (:then_1
            (bind _newtrack_0_2 (Timeline|Timeline_4 PlayFromStart)
              (:Update
                (Variables|Moto|SetBiker_Anim (Math|Float|Lerp (Variables|Moto|GetBiker_Anim) 1e+02 _newtrack_0_2)))))
          (:then_2
            (bind _newtrack_0_3 (Timeline|Timeline_5 PlayFromStart)
              (:Update
                (Variables|Moto|SetF_Wheel (Math|Rotator|Lerp(Rotator) (Variables|Moto|GetF_Wheel) "0, 0,15.000000" _newtrack_0_3))))))))
    (:then_1
      (if (not (!= AxisValue 0.0))
        (Utilities|FlowControl|Sequence
          (:then_0
            (bind _newtrack_0_4 (Timeline|Timeline_6 PlayFromStart)
              (:Update
                (Variables|Moto|SetSteer (Math|Rotator|Lerp(Rotator) (Variables|Moto|GetSteer) "0, 0, 0" _newtrack_0_4)))))
          (:then_1
            (bind _newtrack_0_5 (Timeline|Timeline_7 PlayFromStart)
              (:Update
                (Variables|Moto|SetBiker_Anim (Math|Float|Lerp (Variables|Moto|GetBiker_Anim) 5e+01 _newtrack_0_5)))))
          (:then_2
            (bind _newtrack_0_6 (Timeline|Timeline_8 PlayFromStart)
              (:Update
                (Variables|Moto|SetF_Wheel (Math|Rotator|Lerp(Rotator) (Variables|Moto|GetF_Wheel) "0, 0, 0" _newtrack_0_6))))))))
    (:then_2
      (if (< AxisValue -0.1)
        (Utilities|FlowControl|Sequence
          (:then_0
            (bind _newtrack_0_7 (Timeline|Timeline_9 PlayFromStart)
              (:Update
                (Variables|Moto|SetSteer (Math|Rotator|Lerp(Rotator) (Variables|Moto|GetSteer) "0, 0,-25.000000" _newtrack_0_7)))))
          (:then_1
            (bind _newtrack_0_8 (Timeline|Timeline_10 PlayFromStart)
              (:Update
                (Variables|Moto|SetBiker_Anim (Math|Float|Lerp (Variables|Moto|GetBiker_Anim) 0.0 _newtrack_0_8)))))
          (:then_2
            (bind _newtrack_0_9 (Timeline|Timeline_11 PlayFromStart)
              (:Update
                (Variables|Moto|SetF_Wheel (Math|Rotator|Lerp(Rotator) (Variables|Moto|GetF_Wheel) "0, 0,-15.000000" _newtrack_0_9))))))))))

(event Custom|Server
  ;[1 1 1] 车把上的手
  (CallFunction|Client))

(event Custom|Client
  (bind _mesh (Variables|Character|GetMesh))
  ;[1 1 1] 车把上的手
  (Transformation|SetWorldTransform (Variables|Default|GetHand_Left) (Transformation|GetSocketTransform _mesh "LeftHand" "RTS_World") false false)
  (Transformation|SetWorldTransform (Variables|Default|GetHand_Right) (Transformation|GetSocketTransform _mesh "RightHand" "RTS_World") false false))

(event EventTick
  (params (DeltaSeconds :type Float%20%28single-precision%29))
  (bind _vehiclemovement (Variables|Default|GetVehicleMovement))
  (bind _parking (Variables|Default|GetParking))
  ;[1 0.275 0.275] Parking on/off
  (Utilities|FlowControl|Sequence
    (:then_0
      (if (or (< (Class|WheeledVehicleMovementComponent|GetEngineRotationSpeed _vehiclemovement) 2e+02) (== (Class|WheeledVehicleMovementComponent|GetCurrentGear _vehiclemovement) -1))
        (bind _newtrack_0 (Timeline|Timeline_0 Play)
          (:Update
            (Variables|Moto|SetIdle _newtrack_0)
            (Variables|/Script/Engine.PhysicsThrusterComponent|SetThrustStrength _parking 9e+04)))
        (else
          (Utilities|FlowControl|Sequence
            (:then_0
              (Timeline|Timeline_0 Reverse))
            (:then_1
              (Variables|/Script/Engine.PhysicsThrusterComponent|SetThrustStrength _parking 0.0))))))
    (:then_1
      (|SlowSpeed))
    (:then_2
      (CallFunction|UpdateHUDStrings)
      (CallFunction|SetupIncarHUD))
    (:then_3
      (|GrabHandleBar))
    (:then_4
      (|LaunchProp))
    (:then_5
      (|HandTrack))
    (:then_6
      ;[1 1 1] 车把上的手
      (CallFunction|Server))))

(event EventBeginPlay
  (bind _returnvalue (Class|HeadMountedDisplayFunctionLibrary|IsHeadMountedDisplayEnabled))
  (CallFunction|EnableIncarView _returnvalue)
  (if _returnvalue
    ;[1 1 1] 重置镜头
    (Class|HeadMountedDisplayFunctionLibrary|ResetOrientationandPosition 0.0 "OrientationAndPosition")))

(event Input|ActionEvents|InputActionResetVR
  (params (Key :type Key%20Structure))
  ;[1 1 1] 重置镜头
  (:Pressed
    (Class|HeadMountedDisplayFunctionLibrary|ResetOrientationandPosition 0.0 "OrientationAndPosition")))

(event Input|AxisEvents|InputAxislefthandf
  (params (AxisValue :type Float%20%28single-precision%29))
  ;[1 1 1] vr手部控制
  (Transformation|AddLocalOffset (Variables|/Game/Blueprint/Roles/vrHand.VRHand_C|GetMotionController (Variables|Default|GetLeftController)) (Math|Vector|MakeVector AxisValue 0.0 0.0) false false))

(event Input|AxisEvents|InputAxislefthandr
  (params (AxisValue :type Float%20%28single-precision%29))
  ;[1 1 1] vr手部控制
  (Transformation|AddLocalOffset (Variables|/Game/Blueprint/Roles/vrHand.VRHand_C|GetMotionController (Variables|Default|GetLeftController)) (Math|Vector|MakeVector 0.0 AxisValue 0.0) false false))

(event Input|AxisEvents|InputAxislefthandu
  (params (AxisValue :type Float%20%28single-precision%29))
  ;[1 1 1] vr手部控制
  (Transformation|AddLocalOffset (Variables|/Game/Blueprint/Roles/vrHand.VRHand_C|GetMotionController (Variables|Default|GetLeftController)) (Math|Vector|MakeVector 0.0 0.0 AxisValue) false false))

(event Input|AxisEvents|InputAxisMoveForward
  (params (AxisValue :type Float%20%28single-precision%29))
  ;[0.3937 1 0.39] Move Forward/Back
  (Class|WheeledVehicleMovementComponent|SetThrottleInput (Variables|Default|GetVehicleMovement) AxisValue))

(event Input|AxisEvents|InputAxisrighthandf
  (params (AxisValue :type Float%20%28single-precision%29))
  ;[1 1 1] vr手部控制
  (Transformation|AddLocalOffset (Variables|/Game/Blueprint/Roles/vrHand.VRHand_C|GetMotionController (Variables|Default|GetRightController)) (Math|Vector|MakeVector AxisValue 0.0 0.0) false false))

(event Input|AxisEvents|InputAxisrighthandr
  (params (AxisValue :type Float%20%28single-precision%29))
  ;[1 1 1] vr手部控制
  (Transformation|AddLocalOffset (Variables|/Game/Blueprint/Roles/vrHand.VRHand_C|GetMotionController (Variables|Default|GetRightController)) (Math|Vector|MakeVector 0.0 AxisValue 0.0) false false))

(event Input|AxisEvents|InputAxisrighthandu
  (params (AxisValue :type Float%20%28single-precision%29))
  ;[1 1 1] vr手部控制
  (Transformation|AddLocalOffset (Variables|/Game/Blueprint/Roles/vrHand.VRHand_C|GetMotionController (Variables|Default|GetRightController)) (Math|Vector|MakeVector 0.0 0.0 AxisValue) false false))

(event Input|AxisEvents|InputAxisMoveRight
  (params (AxisValue :type Float%20%28single-precision%29))
  ;[0.3937 1 0.39] Move Left/Right
  (CallFunction|MoveRightS AxisValue))

(event Input|KeyboardEvents|Tab
  (params (Key :type Key%20Structure))
  ;[1 1 1] 切换摄像机
  (:Pressed
    (CallFunction|EnableIncarView (not (Variables|Moto|GetIsInMotor)))
    (CallFunction|ResetVRDevice)))

(fn ConstructionScript)

(fn UpdateHUDStrings
  (Variables|Moto|SetSpeed%20Display%20String (Utilities|String|Append (Utilities|String|ToString(Integer) (Math|Float|Floor (Math|Float|Absolute(Float) (* (Class|WheeledVehicleMovementComponent|GetForwardSpeed (Variables|Default|GetVehicleMovement)) 0.036)))) " km/h")))

(fn EnableIncarView
  (params (State :type Boolean))
  (bind _rightcontroller (Variables|Default|GetRightController))
  (bind _leftcontroller (Variables|Default|GetLeftController))
  (bind _chasecamera (Variables|Default|GetChaseCamera))
  (bind _internalcamera (Variables|Default|GetInternalCamera))
  (bind _biker (Variables|Default|GetBiker))
  (Variables|Moto|SetIsInMotor State)
  (if (Variables|Moto|GetIsInMotor)
    (Components|Activation|Activate _internalcamera false)
    (Components|Activation|Deactivate _chasecamera)
    (Rendering|SetVisibility _biker false false)
    (Utilities|IsValid _rightcontroller
      (:Is%20Valid
        (Rendering|SetVisibility (Variables|/Game/Blueprint/Roles/vrHand.VRHand_C|GetHandMesh _rightcontroller) true false)
        (CallFunction|PrintP "01")))
    (else
      (Components|Activation|Deactivate _internalcamera)
      (Components|Activation|Activate _chasecamera false)
      (Rendering|SetVisibility _biker true false)
      (Utilities|IsValid _leftcontroller
        (:Is%20Valid
          (Rendering|SetVisibility (Variables|/Game/Blueprint/Roles/vrHand.VRHand_C|GetHandMesh _leftcontroller) false false)
          (CallFunction|PrintP "02"))))))

(fn SetupIncarHUD
  (Rendering|Components|TextRender|SetText (Variables|Default|GetSpeed) (Utilities|Text|ToText(String) (Variables|Moto|GetSpeed%20Display%20String))))

(event Custom|SlowClient
  (bind _biker (Variables|Default|GetBiker))
  ;[1 1 1] 减速
  (Rendering|Material|SetMaterial _biker 0 "/Game/Blueprint/Prop/lan.lan")
  (Rendering|Material|SetMaterial _biker 1 "/Game/Blueprint/Prop/lan.lan")
  (Variables|Default|Setslow? true)
  (Utilities|FlowControl|Delay 8.0)
  (Variables|Default|Setslow? false)
  (Rendering|Material|SetMaterial _biker 0 "/Game/Blueprint/Roles/Biker/Materials/M_Body_Red_Biker.M_Body_Red_Biker")
  (Rendering|Material|SetMaterial _biker 1 "/Game/Blueprint/Roles/Biker/Materials/M_Helmet_Red.M_Helmet_Red"))

(event Custom|SlowServer
  ;[1 1 1] 减速
  (CallFunction|SlowClient))

(event Custom|NotRightHandNear_C
  (bind _rightcontroller (Variables|Default|GetRightController))
  (Rendering|SetVisibility (Variables|Default|GetHand_Right) false false)
  (Utilities|IsValid _rightcontroller
    (:Is%20Valid
      (if (Variables|Moto|GetIsInMotor)
        (Rendering|SetVisibility (Variables|/Game/Blueprint/Roles/vrHand.VRHand_C|GetHandMesh _rightcontroller) true false)))))

(event Custom|LeftHandNear_C
  (bind _leftcontroller (Variables|Default|GetLeftController))
  (Rendering|SetVisibility (Variables|Default|GetHand_Left) true false)
  (Utilities|IsValid _leftcontroller
    (:Is%20Valid
      (Rendering|SetVisibility (Variables|/Game/Blueprint/Roles/vrHand.VRHand_C|GetHandMesh _leftcontroller) false false))))

(event Custom|NotRightHandNear_S
  (CallFunction|NotRightHandNearC))

(event Custom|RightHandNear_S
  (CallFunction|RightHandNearC))

(event Custom|NotLeftHandNear_C
  (bind _leftcontroller (Variables|Default|GetLeftController))
  (Rendering|SetVisibility (Variables|Default|GetHand_Left) false false)
  (Utilities|IsValid _leftcontroller
    (:Is%20Valid
      (if (Variables|Moto|GetIsInMotor)
        (Rendering|SetVisibility (Variables|/Game/Blueprint/Roles/vrHand.VRHand_C|GetHandMesh _leftcontroller) true false)))))

(event Custom|LeftHandNear_S
  (CallFunction|LeftHandNearC))

(event Custom|NotLeftHandNear_S
  (CallFunction|NotLeftHandNearC))

(event Custom|RightHandNear_C
  (bind _rightcontroller (Variables|Default|GetRightController))
  (Rendering|SetVisibility (Variables|Default|GetHand_Right) true false)
  (Utilities|IsValid _rightcontroller
    (:Is%20Valid
      (Rendering|SetVisibility (Variables|/Game/Blueprint/Roles/vrHand.VRHand_C|GetHandMesh _rightcontroller) false false))))

(event Custom|MoveLeftHandClient
  (params (DeltaLocation :type Vector) (DeltaRotation :type Rotator))
  (bind _leftcontroller (Variables|Default|GetLeftController))
  (Utilities|IsValid _leftcontroller
    (:Is%20Valid
      (Transformation|SetWorldLocationAndRotation (Variables|/Game/Blueprint/Roles/vrHand.VRHand_C|GetHandScene _leftcontroller) DeltaLocation DeltaRotation false false)
      (if (not (Pawn|IsLocallyControlled))
        (Rendering|SetVisibility (Variables|/Game/Blueprint/Roles/vrHand.VRHand_C|GetHandMesh _leftcontroller) false false)))))

(event Custom|MoveRightHandSever
  (params (DeltaLocation :type Vector) (DeltaRotation :type Rotator))
  (CallFunction|MoveRightHandClient DeltaLocation DeltaRotation))

(event Custom|MoveRightHandClient
  (params (DeltaLocation :type Vector) (DeltaRotation :type Rotator))
  (bind _rightcontroller (Variables|Default|GetRightController))
  (Utilities|IsValid _rightcontroller
    (:Is%20Valid
      (Transformation|SetWorldLocationAndRotation (Variables|/Game/Blueprint/Roles/vrHand.VRHand_C|GetHandScene _rightcontroller) DeltaLocation DeltaRotation false false)
      (if (not (Pawn|IsLocallyControlled))
        (Rendering|SetVisibility (Variables|/Game/Blueprint/Roles/vrHand.VRHand_C|GetHandMesh _rightcontroller) false false)))))

(event Custom|MoveLeftHandSever
  (params (DeltaLocation :type Vector) (DeltaRtation :type Rotator))
  (CallFunction|MoveLeftHandCLient DeltaLocation DeltaRtation))

(event Custom|LeftFireServer
  (params (New%20Rotation :type Rotator) (LaunchSpeed :type Float%20%28single-precision%29))
  (CallFunction|LeftFireClient New%20Rotation LaunchSpeed))

(event Custom|RightFireClient
  (params (NewRotation :type Rotator) (LaunchSpeed :type Float%20%28single-precision%29))
  (bind _rightcontroller (Variables|Default|GetRightController))
  (Utilities|IsValid _rightcontroller
    (:Is%20Valid
      (Variables|/Game/Blueprint/Roles/vrHand.VRHand_C|SetGrioState _rightcontroller "NewEnumerator0")
      (bind _asfire_banana (Utilities|Casting|CastToFire_Banana (Variables|/Game/Blueprint/Roles/vrHand.VRHand_C|GetProp_BP _rightcontroller))
        (:then
          (Transformation|DetachFromActor _asfire_banana "KeepWorld" "KeepWorld" "KeepWorld")
          (Transformation|SetActorRotation _asfire_banana NewRotation)
          (Variables|/Script/Engine.ProjectileMovementComponent|SetInitialSpeed (Variables|/Game/Blueprint/Prop/Fire_Banana.Fire_Banana_C|GetProjectileMovement _asfire_banana) LaunchSpeed)
          (Components|Activation|Activate (Variables|/Game/Blueprint/Prop/Fire_Banana.Fire_Banana_C|GetProjectileMovement _asfire_banana) true))
        (:CastFailed
          (bind _asfire_slow (Utilities|Casting|CastToFire_slow (Variables|/Game/Blueprint/Roles/vrHand.VRHand_C|GetProp_BP _rightcontroller))
            (:then
              (Transformation|DetachFromActor _asfire_slow "KeepWorld" "KeepWorld" "KeepWorld")
              (Transformation|SetActorRotation _asfire_slow NewRotation)
              (Variables|/Script/Engine.ProjectileMovementComponent|SetInitialSpeed (Variables|/Game/Blueprint/Prop/Fire_slow.Fire_slow_C|GetProjectileMovement _asfire_slow) LaunchSpeed)
              (Components|Activation|Activate (Variables|/Game/Blueprint/Prop/Fire_slow.Fire_slow_C|GetProjectileMovement _asfire_slow) true))
            (:CastFailed
              (bind _ashammer (Utilities|Casting|CastToHammer (Variables|/Game/Blueprint/Roles/vrHand.VRHand_C|GetProp_BP _rightcontroller)))
              (Actor|DestroyActor _ashammer)
              (Game|SpawnActorfromClass "/Game/Blueprint/Prop/Fire_Hammer.Fire_Hammer_C" (Math|Transform|MakeTransform (Transformation|GetWorldLocation (Variables|/Game/Blueprint/Roles/vrHand.VRHand_C|GetHandMesh (Variables|Default|GetRightController))) NewRotation "1,1,1") "Undefined" self 0)))))
      (Variables|/Game/Blueprint/Roles/vrHand.VRHand_C|SetProp (Variables|Default|GetRightController) "NewEnumerator6")
      (Variables|/Game/Blueprint/Roles/vrHand.VRHand_C|SetProp_BP (Variables|Default|GetRightController) 0)
      (Variables|Default|SetProp "NewEnumerator6"))))

(event Custom|LeftFireClient
  (params (New%20Rotation :type Rotator) (LaunchSpeed :type Float%20%28single-precision%29))
  (bind _leftcontroller (Variables|Default|GetLeftController))
  (Utilities|IsValid _leftcontroller
    (:Is%20Valid
      (Variables|/Game/Blueprint/Roles/vrHand.VRHand_C|SetGrioState _leftcontroller "NewEnumerator0")
      (bind _asfire_banana (Utilities|Casting|CastToFire_Banana (Variables|/Game/Blueprint/Roles/vrHand.VRHand_C|GetProp_BP _leftcontroller))
        (:then
          (Transformation|DetachFromActor _asfire_banana "KeepWorld" "KeepWorld" "KeepWorld")
          (Transformation|SetActorRotation _asfire_banana New%20Rotation)
          (Variables|/Script/Engine.ProjectileMovementComponent|SetInitialSpeed (Variables|/Game/Blueprint/Prop/Fire_Banana.Fire_Banana_C|GetProjectileMovement _asfire_banana) LaunchSpeed)
          (Components|Activation|Activate (Variables|/Game/Blueprint/Prop/Fire_Banana.Fire_Banana_C|GetProjectileMovement _asfire_banana) true))
        (:CastFailed
          (bind _asfire_slow (Utilities|Casting|CastToFire_slow (Variables|/Game/Blueprint/Roles/vrHand.VRHand_C|GetProp_BP _leftcontroller))
            (:then
              (Transformation|DetachFromActor _asfire_slow "KeepWorld" "KeepWorld" "KeepWorld")
              (Transformation|SetActorRotation _asfire_slow New%20Rotation)
              (Variables|/Script/Engine.ProjectileMovementComponent|SetInitialSpeed (Variables|/Game/Blueprint/Prop/Fire_slow.Fire_slow_C|GetProjectileMovement _asfire_slow) LaunchSpeed)
              (Components|Activation|Activate (Variables|/Game/Blueprint/Prop/Fire_slow.Fire_slow_C|GetProjectileMovement _asfire_slow) true))
            (:CastFailed
              (bind _ashammer (Utilities|Casting|CastToHammer (Variables|/Game/Blueprint/Roles/vrHand.VRHand_C|GetProp_BP _leftcontroller)))
              (Actor|DestroyActor _ashammer)
              (Game|SpawnActorfromClass "/Game/Blueprint/Prop/Fire_Hammer.Fire_Hammer_C" (Math|Transform|MakeTransform (Transformation|GetWorldLocation (Variables|/Game/Blueprint/Roles/vrHand.VRHand_C|GetHandMesh (Variables|Default|GetLeftController))) New%20Rotation "1,1,1") "Undefined" self 0)))))
      (Variables|/Game/Blueprint/Roles/vrHand.VRHand_C|SetProp (Variables|Default|GetLeftController) "NewEnumerator6")
      (Variables|/Game/Blueprint/Roles/vrHand.VRHand_C|SetProp_BP (Variables|Default|GetLeftController) 0)
      (Variables|Default|SetProp "NewEnumerator6"))))

(event Custom|RightFireServer
  (params (NewRotation :type Rotator) (LaunchSpeed :type Float%20%28single-precision%29))
  (CallFunction|RightFireClient NewRotation LaunchSpeed))

(event Input|MouseEvents|LeftMouseButton
  (params (Key :type Key%20Structure))
  (bind _returnvalue (Transformation|GetActorLocation))
  (bind _leftcontroller (Variables|Default|GetLeftController))
  (bind _handscene (Variables|/Game/Blueprint/Roles/vrHand.VRHand_C|GetHandScene _leftcontroller))
  (bind _returnvalue_2 (Transformation|GetWorldLocation _handscene))
  (bind _returnvalue_3 (- _returnvalue_2 _returnvalue))
  (:Pressed
    (CallFunction|LeftFireServer (Math|Rotator|FindLookatRotation (Variables|LaunchProp|GetLeftHandLocation) _returnvalue_3) (+ (Class|WheeledVehicleMovementComponent|GetForwardSpeed (Variables|Default|GetVehicleMovement)) (Variables|Default|GetInitialLaunchSpeed)))
    (Variables|LaunchProp|SetLeftHandLocation _returnvalue_3)))

(event Input|MouseEvents|RightMouseButton
  (params (Key :type Key%20Structure))
  (bind _returnvalue (Transformation|GetActorLocation))
  (bind _rightcontroller (Variables|Default|GetRightController))
  (bind _handscene (Variables|/Game/Blueprint/Roles/vrHand.VRHand_C|GetHandScene _rightcontroller))
  (bind _returnvalue_2 (Transformation|GetWorldLocation _handscene))
  (bind _returnvalue_3 (- _returnvalue_2 _returnvalue))
  (:Pressed
    (CallFunction|RightFireServer (Math|Rotator|FindLookatRotation (Variables|LaunchProp|GetRightHandLocation) _returnvalue_3) (+ (Class|WheeledVehicleMovementComponent|GetForwardSpeed (Variables|Default|GetVehicleMovement)) (Variables|Default|GetInitialLaunchSpeed)))
    (Variables|LaunchProp|SetRightHandLocation _returnvalue_3)))