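; Spwan911 is a trigger actor that spawns a 911 actor when a Sport actor overlaps its Sphere.
; The overlap runs only with authority and passes the Sport's RightController through the CCCCC and SSSSS custom events.
; SSSSS spawns the 911 at a fixed transform 100 units above the world origin, ignoring the controller it receives.
; Disconnected leftovers hold debug prints, a VRHand path and logic to attach the 911 to an AttachPoint.
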(event OnComponentBeginOverlap(Sphere)
  (params (OverlappedComponent :type Primitive%20Component%20Object%20Reference) (OtherActor :type Actor%20Object%20Reference) (OtherComp :type Primitive%20Component%20Object%20Reference) (OtherBodyIndex :type Integer) (bFromSweep :type Boolean) (SweepResult :type Hit%20Result%20Structure%20%28by%20ref%29))
  (Networking|SwitchHasAuthority
    (:Authority
      (bind _assport (Utilities|Casting|CastToSport OtherActor))
      (CallFunction|CCCCC 0 _assport))))

(event Custom|CCCCC
  (params (NewParam :type VR%20Hand%20Object%20Reference) (NewParam2 :type Sport%20Object%20Reference))
  (CallFunction|SSSSS (Variables|/Game/Blueprint/Roles/Sport.Sport_C|GetRightController NewParam2)))

(event Custom|SSSSS
  (params (NewParam :type VR%20Hand%20Object%20Reference))
  (Game|SpawnActorfromClass "/Game/Blueprint/Roles/911.911_C" (Math|Transform|MakeTransform "0.000000, 0,100.000000" "0,0.000000, 0" "1,1,1") "Undefined" 0 0))

(event EventBeginPlay)

(event Collision|EventActorBeginOverlap
  (params (OtherActor :type Actor%20Object%20Reference)))

(event EventTick
  (params (DeltaSeconds :type Float%20%28single-precision%29)))

(fn ConstructionScript)