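; Hammer is a single-use melee prop, held in a VRHand, that hurts another Sport it hits.
; A Box overlap with a Sport other than its owner calls HurtServer on that target.
; It then resets the prop state on the parent VRHand and the Sport holding that hand, and destroys itself if both casts succeed.
; The Server-to-Client event pair is an unused stub.
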(event OnComponentBeginOverlap(Box)
  (params (OverlappedComponent :type Primitive%20Component%20Object%20Reference) (OtherActor :type Actor%20Object%20Reference) (OtherComp :type Primitive%20Component%20Object%20Reference) (OtherBodyIndex :type Integer) (bFromSweep :type Boolean) (SweepResult :type Hit%20Result%20Structure%20%28by%20ref%29))
  (bind _assport (Utilities|Casting|CastToSport OtherActor))
  (if (not (== OtherActor (Components|GetOwner)))
    (Default|HurtServer _assport)
    (bind _asvrhand (Utilities|Casting|CastToVRHand (Actor|GetAttachParentActor)))
    (Variables|/Game/Blueprint/Roles/vrHand.VRHand_C|SetProp_BP _asvrhand 0)
    (Variables|/Game/Blueprint/Roles/vrHand.VRHand_C|SetProp _asvrhand "NewEnumerator6")
    (Variables|/Game/Blueprint/Roles/vrHand.VRHand_C|SetGrioState _asvrhand "NewEnumerator0")
    (bind _assport_2 (Utilities|Casting|CastToSport (Actor|GetAttachParentActor _asvrhand)))
    (Variables|/Game/Blueprint/Roles/Sport.Sport_C|SetProp _assport_2 "NewEnumerator6")
    (Actor|DestroyActor)))

(event Custom|Client
  (params (Object :type Object%20Object%20Reference)))

(event Custom|Server
  (params (Object :type Object%20Object%20Reference))
  (CallFunction|Client Object))

(event EventBeginPlay)

(event Collision|EventActorBeginOverlap
  (params (OtherActor :type Actor%20Object%20Reference)))

(event EventTick
  (params (DeltaSeconds :type Float%20%28single-precision%29)))

(fn ConstructionScript)