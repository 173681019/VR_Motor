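; Fire_slow is a projectile prop that slows a Sport actor it strikes.
; When its Box hits a surface, it spawns an emitter and another actor at the impact point, then destroys itself.
; When the Box overlaps a Sport other than its owner while ProjectileMovement is active, it calls SlowServer on that target, spawns an emitter and destroys itself.
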(event OnComponentBeginOverlap(Box)
  (params (OverlappedComponent :type Primitive%20Component%20Object%20Reference) (OtherActor :type Actor%20Object%20Reference) (OtherComp :type Primitive%20Component%20Object%20Reference) (OtherBodyIndex :type Integer) (bFromSweep :type Boolean) (SweepResult :type Hit%20Result%20Structure%20%28by%20ref%29))
  ;[1 1 1] 空中碰到人
  (if (Components|Activation|IsActive (Variables|Default|GetProjectileMovement))
    (bind _assport (Utilities|Casting|CastToSport OtherActor))
    (if (not (== _assport (Components|GetOwner)))
      (CallFunction|PrintP (Utilities|GetDisplayName OtherActor))
      (Default|SlowServer _assport)
      (Effects|SpawnEmitteratLocation 0 (.Location (Collision|BreakHitResult SweepResult)))
      (Actor|DestroyActor))))

(event OnComponentHit(Box)
  (params (HitComponent :type Primitive%20Component%20Object%20Reference) (OtherActor :type Actor%20Object%20Reference) (OtherComp :type Primitive%20Component%20Object%20Reference) (NormalImpulse :type Vector :default "0, 0, 0") (Hit :type Hit%20Result%20Structure%20%28by%20ref%29))
  (bind _impactpoint (Collision|BreakHitResult Hit))
  ;[1 1 1] 碰到地面
  (Effects|SpawnEmitteratLocation 0 _impactpoint)
  (Game|SpawnActorfromClass "/Game/Blueprint/Prop/Slowwater.Slowwater_C" (Math|Transform|MakeTransform _impactpoint "0, 0, 0" "1,1,1") "Undefined" 0 0)
  (Actor|DestroyActor))

(fn ConstructionScript)