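; Throwable banana hazard that hurts a Sport actor on overlap and then destroys itself.
; Detach releases it from its parent, enables physics on Box, zeroes spin and doubles its linear velocity, ignoring the HandVelocity input.
; Overlaps count only while physics simulates, and the owner is immune until a Box hit sets OnGround.
; Construction sets projectile initial speed; the Server event only forwards to an empty Client event.
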(event OnComponentHit(Box)
  (params (HitComponent :type Primitive%20Component%20Object%20Reference) (OtherActor :type Actor%20Object%20Reference) (OtherComp :type Primitive%20Component%20Object%20Reference) (NormalImpulse :type Vector :default "0, 0, 0") (Hit :type Hit%20Result%20Structure%20%28by%20ref%29))
  (Variables|Default|SetOnGround true))

(event OnComponentBeginOverlap(overloap)
  (params (OverlappedComponent :type Primitive%20Component%20Object%20Reference) (OtherActor :type Actor%20Object%20Reference) (OtherComp :type Primitive%20Component%20Object%20Reference) (OtherBodyIndex :type Integer) (bFromSweep :type Boolean) (SweepResult :type Hit%20Result%20Structure%20%28by%20ref%29))
  (if (Physics|IsSimulatingPhysics (Variables|Default|GetBox) "None")
    (bind _assport (Utilities|Casting|CastToSport OtherActor))
    (if (Variables|Default|GetOnGround)
      (Default|HurtServer _assport :!label _label)
      (Actor|DestroyActor)
      (elif (not (== _assport (Components|GetOwner)))
        (goto _label)))))

(event Custom|Client
  (params (Object :type Sport%20Object%20Reference) (OnGround :type Boolean) (==owner :type Boolean)))

(event Custom|Detach
  (params (HandVelocity :type Vector))
  (bind _box (Variables|Default|GetBox))
  (Physics|SetSimulatePhysics (Variables|Default|GetBox) true)
  (Transformation|DetachFromActor "KeepWorld" "KeepWorld" "KeepWorld")
  (Class|PrimitiveComponent|SetPhysicsAngularVelocityinRadians _box "0, 0, 0" false "None")
  (bind _returnvalue (Physics|GetPhysicsLinearVelocity _box "None"))
  (Physics|SetPhysicsLinearVelocity (Variables|Default|GetBox) (* _returnvalue 2.0) false "None"))

(event Custom|Server
  (params (Object :type Sport%20Object%20Reference) (OnGround :type Boolean) (==owner :type Boolean))
  (CallFunction|Client Object OnGround ==owner))

(event EventBeginPlay)

(event Collision|EventActorBeginOverlap
  (params (OtherActor :type Actor%20Object%20Reference)))

(event EventTick
  (params (DeltaSeconds :type Float%20%28single-precision%29)))

(fn ConstructionScript
  (Variables|/Script/Engine.ProjectileMovementComponent|SetInitialSpeed (Variables|Default|GetProjectileMovement) (Variables|Default|GetMySetInitialSpeed)))