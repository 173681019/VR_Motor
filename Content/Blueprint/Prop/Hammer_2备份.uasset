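; Backup copy of a hammer prop that a Sport character carries and hits other Sport characters with.
; When its Box overlaps a Sport other than its owner, it calls Hurt on that target, sets the owner's Prop enum and destroys itself, provided the owner is a Sport.
; A Drop event turns on physics for the Box and detaches the hammer, keeping its world transform.
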(event OnComponentBeginOverlap(Box)
  (params (OverlappedComponent :type Primitive%20Component%20Object%20Reference) (OtherActor :type Actor%20Object%20Reference) (OtherComp :type Primitive%20Component%20Object%20Reference) (OtherBodyIndex :type Integer) (bFromSweep :type Boolean) (SweepResult :type Hit%20Result%20Structure%20%28by%20ref%29))
  (bind _assport (Utilities|Casting|CastToSport OtherActor))
  (if (not (== OtherActor (Components|GetOwner)))
    (Default|Hurt _assport)
    (bind _assport_2 (Utilities|Casting|CastToSport (Components|GetOwner)))
    (Variables|/Game/Blueprint/Roles/Sport.Sport_C|SetProp _assport_2 "NewEnumerator6")
    (Actor|DestroyActor)))

(event Custom|Drop
  (Physics|SetSimulatePhysics (Variables|Default|GetBox) true)
  (Transformation|DetachFromActor "KeepWorld" "KeepWorld" "KeepWorld"))

(event EventBeginPlay)

(event Collision|EventActorBeginOverlap
  (params (OtherActor :type Actor%20Object%20Reference)))

(event EventTick
  (params (DeltaSeconds :type Float%20%28single-precision%29)))

(fn ConstructionScript)