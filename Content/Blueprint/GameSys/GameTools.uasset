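; GameTools is a collection of shared helper functions for debug printing, VR detection, vector math, percent-chance rolls, screen effects and a version string.
; Debug prints use random colors and are gated by IsDebug, which is hardcoded to false.
; FlashScreen pairs a brief white camera fade with a shake, TweenScreen runs a slower black fade, and CheckInAir uses a short downward trace.
; Random rolls are unsynchronized, with a note to synchronize them for network play.
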(fn PrintP
  (params (String :type String))
  (if (Config|IsDebug)
    (Development|PrintString 0 String true true (Utilities|Struct|MakeLinearColor (Math|Random|RandomFloat) (Math|Random|RandomFloat) (Math|Random|RandomFloat) 1.0) 11111.0)))

(fn CheckifForward
  (params (S :type Actor%20Object%20Reference%20%28by%20ref%29) (T :type Actor%20Object%20Reference%20%28by%20ref%29))
  (return (> (Class|Actor|GetDotProductto S T) 0.0)))

(fn IsVrMode
  (return (Class|HeadMountedDisplayFunctionLibrary|IsHeadMountedDisplayConnected)))

(fn PrintStringMultiple
  (params (String :type String) (Times :type Integer))
  (for _index (range 0 Times)
    (CallFunction|PrintP String)))

(fn ShakeCamera
  (Class|PlayerController|ClientPlayCameraShake (Game|GetPlayerController 0) 0 1.0 "CameraLocal" "0, 0, 0"))

(fn GetVectorDistance
  (params (V1 :type Vector) (V2 :type Vector))
  (return (Math|Vector|VectorLength (- V1 V2))))

(fn GetRandom
  (params (seed :type Integer))
  ;[1 1 1] 计算出有多少概率触发某事，在网络模式下，此方法应改为同步
  (return (< (Math|Random|RandomInteger 100) seed)))

(fn CheckinAir?
  (params (OriPoint :type Vector))
  (bind _returnvalue (Collision|LineTraceForObjects 0 OriPoint (+ OriPoint "0, 0,-170.000000") (LocalVariables|GetObjectType) false 0 "None"))
  (return (not _returnvalue)))

(fn FlashScreen
  (CameraFades|StartCameraFade (Game|GetPlayerCameraManager 0) 1.0 0.0 0.1 "(R=1.000000,G=1.000000,B=1.000000,A=1.000000)" false false)
  (CallFunction|ShakeCamera))

(fn IsDebug
  (return false))

(fn TweenScreen
  (CameraFades|StartCameraFade (Game|GetPlayerCameraManager 0) 3.0 0.0 3.0 "(R=0.000000,G=0.000000,B=0.000000,A=1.000000)" false false))

(fn GetVersion
  (return "Beta 2.1"))