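; Game mode for a multiplayer Sport race that runs spawning, countdown, finish and leaderboard.
; PostLogin spawns pawns at TargetPoints after a delay; Tick starts the countdown and unlocks movement once all players spawn.
; endgame stops each finisher, recursively ranks a descending score into five widget-seeded entries and saves them.
; When all finish, leaderboards attach to each pawn's UIPoint; the save-loading check is unwired.
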(event Custom|Make
  (bind _ui数组 (Variables|Default|GetUI数组))
  ;[1 1 1] 排行榜
  (if (<= (Variables|Default|Get排名数) 4)
    (if (> (Variables|Default|Get分数) (.Value (Utilities|Struct|Break排名_UDS (Utilities|Array|Get(acopy) (Variables|Default|GetUI数组) (Variables|Default|Get排名数)))))
      (Utilities|Array|Insert _ui数组 (Utilities|Struct|Make排名_UDS (Variables|Default|Get名称) (Variables|Default|Get分数)) (Variables|Default|Get排名数))
      (Utilities|Array|RemoveIndex _ui数组 (- (Utilities|Array|Length _ui数组) 1))
      (elif (== (Variables|Default|Get分数) (.Value (Utilities|Struct|Break排名_UDS (Utilities|Array|Get(acopy) (Variables|Default|GetUI数组) (Variables|Default|Get排名数)))))
        (Utilities|Array|SetArrayElem (Variables|Default|GetUI数组) (Variables|Default|Get排名数) (Utilities|Struct|Make排名_UDS (Variables|Default|Get名称) (Variables|Default|Get分数)))
        (else
          (Variables|Default|Set排名数 (+ (Variables|Default|Get排名数) 1))
          (CallFunction|Make))))))

(event Custom|LoadSave
  ;[1 1 1] 排行榜
  (bind _returnvalue (SaveGame|LoadGamefromSlot (Variables|Default|Get保存名称)))
  (bind _as排名_save (Utilities|Casting|CastTo排名_Save _returnvalue))
  (bind _output_get (Variables|Default|Set保存 _as排名_save))
  (Variables|Default|SetUI数组 (Variables|/Game/UI/排名/排名_Save.排名_Save_C|GetQst _output_get)))

(event Custom|SaveGame
  ;[1 1 1] 排行榜
  (bind _returnvalue (SaveGame|CreateSaveGameObject "/Game/UI/排名/排名_Save.排名_Save_C"))
  (bind _output_get (Variables|Default|Set保存 _returnvalue))
  (Variables|/Game/UI/排名/排名_Save.排名_Save_C|SetQst _output_get (Variables|Default|GetUI数组))
  (SaveGame|SaveGametoSlot _output_get (Variables|Default|Get保存名称)))

(event Custom|endgame
  (params (Sport :type Sport%20Object%20Reference))
  (bind _returnvalue (Utilities|GetDisplayName Sport))
  (bind _uipoint (Variables|/Game/Blueprint/Roles/Sport.Sport_C|GetUIPoint Sport))
  (if (not (Utilities|Enum|Equal(Enum) (Variables|Default|Get名称) _returnvalue))
    (bind _returnvalue_2 (Game|SpawnActorfromClass "/Game/UI/UI/完成_bp.完成_bp_C" (Transformation|GetWorldTransform _uipoint) "Undefined" 0 0))
    (Transformation|AttachComponentToComponent _returnvalue_2 _uipoint "None" "SnapToTarget" "SnapToTarget" "SnapToTarget" true)
    (Variables|/Game/Blueprint/Roles/Sport.Sport_C|SetCanMoveMotor Sport false)
    (Variables|Default|SetEndGamePlayerNum (+ (Variables|Default|GetEndGamePlayerNum) 1))
    (Variables|Default|Set名称 _returnvalue)
    (Variables|Default|Set排名数 0)
    (CallFunction|Make)
    (Variables|Default|Set分数 (- (Variables|Default|Get分数) 2e+02))
    (CallFunction|SaveGame)))

(event EventBeginPlay
  (bind _outactors (Actor|GetAllActorsOfClass "/Script/Engine.TargetPoint")) ; Find the player starts in the level
  (Variables|Default|SetStartPoint _outactors)
  (for _index (range 1 5)
    (bind _returnvalue (UserInterface|CreateWidget "/Game/UI/排名/排名_显示.排名_显示_C"))
    (Utilities|Array|Add (Variables|Default|GetUI数组) (Utilities|Struct|Make排名_UDS (Variables|/Game/UI/排名/排名_显示.排名_显示_C|Get昵称 _returnvalue) (Math|Conversions|ToFloat(Integer) (Variables|/Game/UI/排名/排名_显示.排名_显示_C|Get分数 _returnvalue))))))

(event EventOnLogout
  (params (ExitingController :type Controller%20Object%20Reference)))

(event EventPostLogin
  (params (NewPlayer :type Player%20Controller%20Object%20Reference))
  ;[1 1 1] PostLogin会在BeginPlay之后执行，强行延时执行是一个办法,但也可以在别处初始化数据
  (Utilities|FlowControl|Delay 1.0)
  (bind _returnvalue (Game|SpawnActorfromClass "/Game/Blueprint/Roles/Sport.Sport_C" (Transformation|GetActorTransform (Utilities|Array|Get(acopy) (Variables|Default|GetStartPoint) (Variables|Default|Getspawn%20order))) "AlwaysSpawn" 0 (Variables|Default|Getspawn%20order) 0)) ; Spawn a pawn at the specified player start
  (Variables|Default|Setspawn%20order (+ (Variables|Default|Getspawn%20order) 1))
  (Default|InitController _returnvalue NewPlayer))

(event EventTick
  (params (DeltaSeconds :type Float%20%28single-precision%29))
  (Utilities|FlowControl|Sequence
    (:then_0
      ;[1 1 1] 游戏开始
      (if (== (Variables|Default|Getspawn%20order) (Variables|Default|GetPlayGamePlayerNum))
        (Utilities|FlowControl|DoOnce false
          (:Completed
            (Utilities|FlowControl|Delay 3.0)
            (bind _outactors (Actor|GetAllActorsOfClass "/Game/Blueprint/Roles/Sport.Sport_C"))
            (for _array_element _outactors
              (bind _returnvalue (Game|SpawnActorfromClass "/Game/UI/UI/倒计时_bp.倒计时_bp_C" (Transformation|GetWorldTransform (Variables|/Game/Blueprint/Roles/Sport.Sport_C|GetUIPoint _array_element)) "Undefined" 0 0))
              (Transformation|AttachComponentToComponent _returnvalue (Variables|/Game/Blueprint/Roles/Sport.Sport_C|GetUIPoint _array_element) "None" "SnapToTarget" "SnapToTarget" "SnapToTarget" true))
            (Utilities|FlowControl|Delay 3.0)
            (bind _outactors_2 (Actor|GetAllActorsOfClass "/Game/Blueprint/Roles/Sport.Sport_C"))
            (for _array_element_2 _outactors_2
              (Variables|/Game/Blueprint/Roles/Sport.Sport_C|SetCanMoveMotor _array_element_2 true))))))
    (:then_1
      (if (== (Variables|Default|GetEndGamePlayerNum) (Variables|Default|GetPlayGamePlayerNum))
        (Utilities|FlowControl|DoOnce false
          (:Completed
            (Utilities|FlowControl|Delay 3.0)
            (bind _outactors_3 (Actor|GetAllActorsOfClass "/Game/Blueprint/Roles/Sport.Sport_C"))
            (for _array_element_3 _outactors_3
              (bind _returnvalue_2 (Game|SpawnActorfromClass "/Game/UI/排名/排名_BP.排名_BP_C" (Transformation|GetWorldTransform (Variables|/Game/Blueprint/Roles/Sport.Sport_C|GetUIPoint _array_element_3)) "Undefined" 0 (Variables|Default|GetUI数组) 0))
              (Transformation|AttachComponentToComponent _returnvalue_2 (Variables|/Game/Blueprint/Roles/Sport.Sport_C|GetUIPoint _array_element_3) "None" "SnapToTarget" "SnapToTarget" "SnapToTarget" true))))))))

(fn ConstructionScript)