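; Game instance that handles LAN session matchmaking and controller vibration.
; MatchGame searches sessions and joins the first with a free player slot, otherwise or on failure calling CreateRoom.
; CreateRoom creates a four-connection LAN session and opens the waiting map as a listen server.
; HandShake plays brief force feedback: Left drives only the left large motor, any other hand value drives the other three.
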(event Custom|CreateRoom
  (|Session (Game|GetPlayerController 0) 4 true
    (:OnSuccess
      (Game|OpenLevel(byName) (Variables|Default|GetWaitingMapName) true "listen"))))

(event Custom|JoinGame
  (params (SearchResult :type Blueprint%20Session%20Result%20Structure%20%28by%20ref%29))
  (|JoinSession (Game|GetPlayerController 0) SearchResult))

(event Custom|MatchGame
  (Variables|Default|SetCurrentSession "")
  (Variables|Default|SetFindOne false)
  (bind _results (|FindSessions (Game|GetPlayerController 0) 99 true)
    (:OnSuccess
      (CallFunction|PrintP (Utilities|String|Append "房间数" (Utilities|String|ToString(Integer) (Utilities|Array|Length _results))))
      (bind _array_element (Utilities|Array|ForEachLoopwithBreak _results :!label _label)
        (:LoopBody
          (if (< (Class|FindSessionsCallbackProxy|GetCurrentPlayers _array_element) (Class|FindSessionsCallbackProxy|GetMaxPlayers _array_element))
            (Variables|Default|SetCurrentSession _array_element)
            (Variables|Default|SetFindOne true)
            (goto _label Break)))
        (:Completed
          (if (Variables|Default|GetFindOne) :!label _label_2
            (CallFunction|JoinGame (Variables|Default|GetCurrentSession))
            (CallFunction|PrintP "加入房间")
            (else
              (CallFunction|CreateRoom)
              (CallFunction|PrintP "创建房间"))))))
    (:OnFailure
      (goto _label_2))))

(event Custom|HandShake
  (params (Index :type EControllerHand%20Enum :default "Left") (Intensity :type Float%20%28single-precision%29))
  (bind _returnvalue (Utilities|Select :Index Index :Left true :Right false :AnyHand false :Pad false :ExternalCamera false :Gun false :Special_1 false :Special_2 false :Special_3 false :Special_4 false :Special_5 false :Special_6 false :Special_7 false :Special_8 false :Special_9 false :Special_10 false :Special_11 false))
  (bind _returnvalue_2 (not _returnvalue))
  (Game|Feedback|PlayDynamicForceFeedback (Game|GetPlayerController 0) Intensity 0.15 _returnvalue _returnvalue_2 _returnvalue_2 _returnvalue_2))